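; Player controller for the Hackerman character that toggles entering and exiting a computer with the 1 key.
; It reads the pawn's ComputerInFocus, tracks state in InComputer, and calls EnterComputer or ExitComputer on that computer, passing itself.
; Entering requires a valid focused computer, while exiting skips that check.
; Author comments note that the key cannot exit in UI-only input mode.
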(event `Key|One`
  (params (Key :type "Key Structure"))
  (bind _returnvalue (`GameplayStatics.GetPlayerPawn` 0))
  (:`Pressed`
    (if (`self.InComputer`)
      (bind _asbp_hackerman (cast `/Game/Characters/Player/BP_Hackerman` _returnvalue))
      (set `self.InComputer` false)
      (`/Game/Blueprints/ComputerSystem/BP_ComputerSystem.ExitComputer` (`/Game/Characters/Player/BP_Hackerman.ComputerInFocus` _asbp_hackerman) self) ; If you somehow move out of the collider while in UI only this will be some undefined behavior
      (else
        (bind _asbp_hackerman_2 (cast `/Game/Characters/Player/BP_Hackerman` _returnvalue))
        (bind _computerinfocus (`/Game/Characters/Player/BP_Hackerman.ComputerInFocus` _asbp_hackerman_2))
        (`/Engine/EditorBlueprintResources/StandardMacros.IsValid` _computerinfocus
          (:`Is Valid`
            (set `self.InComputer` true)
            (`/Game/Blueprints/ComputerSystem/BP_ComputerSystem.EnterComputer` _computerinfocus self)))))))

(fn `UserConstructionScript`)