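; Camera console actor that cycles through camera views automatically, with a brief distortion effect on its display plane at each switch.
; A looping timer set on BeginPlay drives the cycling, which always steps to the right.
; Each switch enables distortion, calls CycleCamera and disables distortion after a short delay.
; The effect toggles a scalar parameter through a dynamic material instance created on every toggle.
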(event `self.ReceiveBeginPlay`
  (`KismetSystemLibrary.K2_SetTimerDelegate` (`|CreateDelegate` :!event `CycleCameras`) 2.0 true))

(event `CycleCameras`
  (`self.ToggleDistortion` true)
  (`self.CycleCamera` "RIGHT")
  (`KismetSystemLibrary.Delay` 0.2)
  (`self.ToggleDistortion` false))

(event `ToggleDistortion`
  (params (Enabled :type Boolean))
  (bind _plane (`self.Plane`))
  (bind _returnvalue (`PrimitiveComponent.CreateDynamicMaterialInstance` _plane 0 (`PrimitiveComponent.GetMaterial` _plane 0) "None"))
  (`MaterialInstanceDynamic.SetScalarParameterValue` _returnvalue "PlayDistortion" (`KismetMathLibrary.SelectFloat` 1.0 0.0 Enabled))
  (`PrimitiveComponent.SetMaterial` (`self.Plane`) 0 _returnvalue))

(fn `UserConstructionScript`)